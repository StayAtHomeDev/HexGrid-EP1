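; BP_Tile is a tile actor whose static mesh gets a randomized color with a glow animation.
; The construction script stores random red and green factors, then applies an initial color from separate random rolls, with blue held at full.
; On BeginPlay a timeline starts at a random time to vary the phase between tiles, and its Glow track scales those factors into the material's Color parameter.
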(event EventBeginPlay
  (Components|Timeline|SetNewTime (Variables|Default|GetTimeline_0) (Math|Random|RandomFloatinRange 0.0 5.0))
  (bind _glow (Timeline|Timeline_0 Play)
    (:Update
      (Rendering|Material|SetVectorParameterValueonMaterials (Variables|Default|GetStaticMesh) "Color" (Math|Vector|MakeVector (* _glow (Variables|Default|GetRandom%20R)) (* _glow (Variables|Default|GetRandom%20G)) 1.0)))))

(fn ConstructionScript
  (bind _returnvalue (Math|Random|RandomFloat))
  (bind _returnvalue_2 (Math|Random|RandomFloat))
  (Variables|Default|SetRandom%20R _returnvalue)
  (Variables|Default|SetRandom%20G _returnvalue_2)
  (Rendering|Material|SetVectorParameterValueonMaterials (Variables|Default|GetStaticMesh) "Color" (Math|Vector|MakeVector _returnvalue _returnvalue_2 1.0)))