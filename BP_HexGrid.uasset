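; BP_HexGrid is an actor that lays out a Width by Height grid of hexagonal tiles in its construction script.
; Spacing derives from the tile mesh's bounding box, Scale and Offset, with a FlipFlop shifting alternate rows by one radius to interlock the hexes.
; An Instanced flag selects either instances on one InstancedStaticMesh or BP_Tile child actors, which receive the mesh through a BP_HexTile cast.
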(event EventBeginPlay)

(event Collision|EventActorBeginOverlap
  (params (OtherActor :type Actor%20Object%20Reference)))

(event EventTick
  (params (DeltaSeconds :type Float%20%28single-precision%29)))

(fn ConstructionScript
  (Components|StaticMesh|SetStaticMesh (Variables|Default|GetInstancedStaticMesh) (Variables|GridOptions|GetTileMesh))
  (Variables|Default|SetRadius (* (.x (.max (StaticMesh|GetBoundingBox (Variables|GridOptions|GetTileMesh)))) (Variables|GridOptions|GetScale)))
  ;[1 1 1] Height Loop
  (for _index (range 0 (- (Variables|GridOptions|GetHeight) 1))
    ;[1 1 1] Width Loop
    (for _index_2 (range 0 (- (Variables|GridOptions|GetWidth) 1))
      (if (Variables|GridOptions|GetInstanced?)
        ;[1 1 1] Instanced Mesh
        (Components|InstancedStaticMesh|AddInstance (Variables|Default|GetInstancedStaticMesh) (Math|Transform|MakeTransform (Math|Vector|MakeVector (+ (* _index_2 (Variables|Default|GetRadius) 2.0) (* _index_2 (Variables|GridOptions|GetOffset)) (Variables|Default|GetRowOffset)) (+ (* (/ (* (Variables|Default|GetRadius) 2.0) (Math|Float|Sqrt 3.0)) 1.5 _index) (* _index (Variables|GridOptions|GetOffset))) 0.0) "0, 0, 0" (Math|Conversions|ToVector(Float) (Variables|GridOptions|GetScale))) false)
        (else
          ;[1 1 1] Child Actors
          (bind _returnvalue (AddComponent|AddChildActorComponent false (Math|Transform|MakeTransform (Math|Vector|MakeVector (+ (* _index_2 (Variables|Default|GetRadius) 2.0) (* _index_2 (Variables|GridOptions|GetOffset)) (Variables|Default|GetRowOffset)) (+ (* (/ (* (Variables|Default|GetRadius) 2.0) (Math|Float|Sqrt 3.0)) 1.5 _index) (* _index (Variables|GridOptions|GetOffset))) 0.0) "0, 0, 0" (Math|Conversions|ToVector(Float) (Variables|GridOptions|GetScale)))))
          (ChildActorComponent|SetChildActorClass _returnvalue "/Game/HexGridSystem/HexGridTut/BP_Tile.BP_Tile_C")
          (bind _asbp_hex_tile (Utilities|Casting|CastToBP_HexTile (Variables|/Script/Engine.ChildActorComponent|GetChildActor _returnvalue)))
          (Components|StaticMesh|SetStaticMesh (Variables|/Game/HexGridSystem/BP_HexTile.BP_HexTile_C|GetHexTile _asbp_hex_tile) (Variables|GridOptions|GetTileMesh)))))
    (Utilities|FlowControl|FlipFlop
      (:A
        (Variables|Default|SetRowOffset (* (Variables|Default|GetRadius) -1.0)))
      (:B
        (Variables|Default|SetRowOffset 0.0)))))